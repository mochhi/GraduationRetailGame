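; BP_NPCManager is a manager Blueprint that tracks the level's NPCs and hands out random NPC points.
; On BeginPlay it caches every BP_NPCPoint and BP_NewNPC actor into arrays.
; GetRandomNPCPoint picks a random cached point.
; GetRandomNPCPointExcluding rerolls only once on a match, so it can still return the excluded point.
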(event `self.ReceiveBeginPlay`
  (bind _outactors (`GameplayStatics.GetAllActorsOfClass` "/Game/Blueprints/BP_NPCPoint.BP_NPCPoint_C"))
  (set `self.NPCPoints` _outactors)
  (bind _outactors_2 (`GameplayStatics.GetAllActorsOfClass` "/Game/Blueprints/BP_NewNPC.BP_NewNPC_C"))
  (set `self.NPC's` _outactors_2))

(fn `GetRandomNPCPoint`
  (returns (RandomPoint :type "/Game/Blueprints/BP_NPCPoint Object Reference"))
  (bind _npcpoints (`self.NPCPoints`))
  (return (`|GetArrayItem` _npcpoints (`KismetMathLibrary.RandomIntegerInRange` 0 (- (`KismetArrayLibrary.Array_Length` _npcpoints) 1)))))

(fn `GetRandomNPCPointExcluding`
  (params (ExcludedPoint :type "Actor Object Reference"))
  (returns (RandomPoint :type "Actor Object Reference"))
  (bind _randompoint (`self.GetRandomNPCPoint`))
  (if (== _randompoint ExcludedPoint)
    (bind _randompoint_2 (`self.GetRandomNPCPoint`))
    (return _randompoint_2)
    (else
      (return _randompoint))))

(fn `UserConstructionScript`)