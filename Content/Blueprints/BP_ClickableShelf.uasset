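; Clickable shelf actor for the SchappenVinden (shelf-finding) game, showing lock, hover and selection state.
; Locked and unlocked states swap the mesh material, while hover and selection flags feed UpdateOutline, which sets an overlay outline material.
; Selection outline overrides hover, except during the manager's unlock phase.
; Cursor hover starts only while clickable; exposed functions set clickability, selection and hold-ring visibility, with no click handling in this Blueprint.
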(event `self.ReceiveBeginPlay`
  (bind _returnvalue (`GameplayStatics.GetActorOfClass` "/Game/Blueprints/BP_SchappenVindenManager.BP_SchappenVindenManager_C"))
  (set `self.SchappenVindenManagerRef` _returnvalue)
  (bind _returnvalue_2 (`GameplayStatics.GetActorOfClass` "/Game/Blueprints/PlayerControllerMain.PlayerControllerMain_C"))
  (set `self.PlayerControllerRef` _returnvalue_2))

(event `self.ReceiveActorBeginCursorOver`
  (if (`self.bIsClickable`)
    (`self.OnHoverStart`)))

(event `self.ReceiveActorEndCursorOver`
  (`self.OnHoverEnd`))

(fn `OnHoverEnd`
  (set `self.IsHovered` false)
  (`self.UpdateOutline`))

(fn `OnHoverStart`
  (set `self.IsHovered` true)
  (`self.UpdateOutline`))

(fn `SetClickable`
  (params (NewClickable :type Boolean))
  (set `self.bIsClickable` NewClickable)
  (if (not NewClickable)
    (`MeshComponent.SetOverlayMaterial` (`self.ShelfMesh`) null)))

(fn `SetShelfDeselected`
  (set `self.IsSelected` false)
  (`self.UpdateOutline`))

(fn `SetShelfLocked`
  (`PrimitiveComponent.SetMaterial` (`self.ShelfMesh`) 0 (`self.LockedMaterial`)))

(fn `SetShelfSelected`
  (set `self.IsSelected` true)
  (`self.UpdateOutline`))

(fn `SetShelfUnlocked`
  (`PrimitiveComponent.SetMaterial` (`self.ShelfMesh`) 0 (`self.UnlockedMaterial`)))

(fn `ShowLoadingRing`
  (params (bVisible :type Boolean))
  (`SceneComponent.SetVisibility` (`self.HoldRingComponent`) bVisible false))

(fn `UpdateOutline`
  (if (and (`self.IsSelected`) (not (`/Game/Blueprints/BP_SchappenVindenManager.bIsUnlockPhase` (`self.SchappenVindenManagerRef`))))
    (`MeshComponent.SetOverlayMaterial` (`self.ShelfMesh`) "/Game/Assets/M_OutlineSelect.M_OutlineSelect")
    (elif (`self.IsHovered`)
      (`MeshComponent.SetOverlayMaterial` (`self.ShelfMesh`) "/Game/Assets/M_OutlineHover.M_OutlineHover")
      (else
        (`MeshComponent.SetOverlayMaterial` (`self.ShelfMesh`) null)))))

(fn `UserConstructionScript`)