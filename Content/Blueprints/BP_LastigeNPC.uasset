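; BP_LastigeNPC is the difficult-customer ("lastige klant") NPC that walks to a set point and can be clicked to start a conversation.
; It caches its managers and target point, randomizes walk speed, and uses AIMoveTo when WalkToTargetPoint is called.
; On arrival it aligns to the point, shows a manager intro row and becomes clickable.
; Capsule cursor events toggle an outline overlay; clicking starts the customer dialogue and removes the tutorial widget.
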(event `self.ReceiveBeginPlay`
  (bind _returnvalue (`GameplayStatics.GetActorOfClass` "/Game/Blueprints/BP_NPCManager.BP_NPCManager_C"))
  (set `self.NPCManagerRef_0` _returnvalue)
  (bind _returnvalue_2 (`GameplayStatics.GetActorOfClass` "/Game/Blueprints/BP_PointLastige.BP_PointLastige_C"))
  (set `self.TargetPoint` _returnvalue_2)
  (bind _returnvalue_3 (`GameplayStatics.GetActorOfClass` "/Game/Blueprints/BP_LastigeKlantManager.BP_LastigeKlantManager_C"))
  (set `self.LastigeKlantManagerRef` _returnvalue_3)
  (set `CharacterMovementComponent.MaxWalkSpeed` (`KismetMathLibrary.RandomFloatInRange` 120.0 150.0) (`self.CharacterMovement`)))

(event `WalkToTargetPoint`
  (`|AIMoveTo` self (`self.K2_GetActorLocation` (`self.TargetPoint`)) null 50.0
    (:`OnSuccess`
      (`self.K2_SetActorRotation` (`self.K2_GetActorRotation` (`self.TargetPoint`)))
      (`self.OnLastigeNPCReachedTarget`)
      (set `self.CanBeClicked` true))))

(event `OnLastigeNPCReachedTarget`
  (`/Game/Blueprints/BP_LastigeKlantManager.ShowManagwerRow` (`self.LastigeKlantManagerRef`) "Intro_02"))

(event `self.CapsuleComponent.OnClicked`
  (params (TouchedComponent :type "PrimitiveComponent Object Reference") (ButtonPressed :type "Key Structure"))
  (bind _lastigeklantmanagerref (`self.LastigeKlantManagerRef`))
  (if (`self.CanBeClicked`)
    (`MeshComponent.SetOverlayMaterial` (`self.Mesh`) null)
    (`/Game/Blueprints/BP_LastigeKlantManager.StartCustomerDialogue` _lastigeklantmanagerref)
    (`Widget.RemoveFromParent` (`/Game/Blueprints/BP_LastigeKlantManager.ManagerTutorialWidget` _lastigeklantmanagerref))
    (set `self.IsHavingConversation` true)))

(event `self.CapsuleComponent.OnBeginCursorOver`
  (params (TouchedComponent :type "PrimitiveComponent Object Reference"))
  (if (`self.CanBeClicked`)
    (`MeshComponent.SetOverlayMaterial` (`self.Mesh`) "/Game/Assets/M_OutlineHover.M_OutlineHover")))

(event `self.CapsuleComponent.OnEndCursorOver`
  (params (TouchedComponent :type "PrimitiveComponent Object Reference"))
  (`MeshComponent.SetOverlayMaterial` (`self.Mesh`) null))

(fn `UserConstructionScript`)