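; A clickable customer NPC for the SchappenVinden shelf-finding task that presents a customer request.
; On BeginPlay it finds BP_SchappenVindenManager and loads request text and target category from a data table row.
; Clicking it while no request is active hands both values to the manager and shows the request widget.
; Hovering applies an outline overlay; Activate and Deactivate functions toggle visibility and collision.
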(event `self.ReceiveBeginPlay`
  (bind _returnvalue (`GameplayStatics.GetActorOfClass` "/Game/Blueprints/BP_SchappenVindenManager.BP_SchappenVindenManager_C"))
  (set `self.SchappenVindenManagerRef` _returnvalue)
  (`self.LoadRequestFromDataTable`))

(event `self.NPC.OnClicked`
  (params (TouchedComponent :type "PrimitiveComponent Object Reference") (ButtonPressed :type "Key Structure"))
  (bind _schappenvindenmanagerref (`self.SchappenVindenManagerRef`))
  (if (not (`/Game/Blueprints/BP_SchappenVindenManager.bRequestActive` (`self.SchappenVindenManagerRef`)))
    (set `/Game/Blueprints/BP_SchappenVindenManager.bRequestActive` true _schappenvindenmanagerref)
    (set `/Game/Blueprints/BP_SchappenVindenManager.ActiveRequestText` (`self.CurrentRequestText`) _schappenvindenmanagerref)
    (set `/Game/Blueprints/BP_SchappenVindenManager.ActiveTargetCategory` (`self.CurrentTargetCategory`) _schappenvindenmanagerref)
    (`self.CreateCustomerRequestWidget`)))

(event `self.ReceiveActorBeginCursorOver`
  (`MeshComponent.SetOverlayMaterial` (`self.NPC`) "/Game/Assets/M_Outline.M_Outline"))

(event `self.ReceiveActorEndCursorOver`
  (`MeshComponent.SetOverlayMaterial` (`self.NPC`) null))

(fn `ActivateCustomer`
  (`self.SetActorHiddenInGame` false)
  (`self.SetActorEnableCollision` true))

(fn `CreateCustomerRequestWidget`
  (bind _returnvalue (`|CreateWidget` "/Game/Blueprints/Widgets/WBP_CustomerRequest.WBP_CustomerRequest_C" null (`self.CurrentRequestText`)))
  (bind _output_get (set `/Game/Blueprints/BP_SchappenVindenManager.CustomerRequestWidgetRef` _returnvalue (`self.SchappenVindenManagerRef`)))
  (`UserWidget.AddToViewport` _output_get 0))

(fn `DeactivateCustomer`
  (`self.SetActorHiddenInGame` true)
  (`self.SetActorEnableCollision` false))

(fn `LoadRequestFromDataTable`
  (bind _returnvalue (`|GetDataTableRow` (`self.CustomerRequestDataTable`) (`self.RequestRowName`))
    (:`then`
      (bind (_requestid _requesttext _targetcategory) (break `/Game/Blueprints/DataTables/ST_CustomerRequest` _returnvalue))
      (set `self.CurrentRequestText` _requesttext)
      (set `self.CurrentTargetCategory` _targetcategory)
      (set `self.bRequestAssigned` true))))

(fn `UserConstructionScript`)