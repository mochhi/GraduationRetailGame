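; BP_LastigeKlantManager sets up the UI and view for what its name suggests is a difficult-customer (lastige klant) dialogue scenario.
; On BeginPlay it adds the dialogue and manager feedback widgets to the viewport, hides the feedback, switches the view to its Camera and hides the player character.
; It also creates a collapsed M1 end screen once, which ShowEndingScreen later makes visible.
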(event `self.ReceiveBeginPlay`
  (bind _returnvalue (`|CreateWidget` "/Game/Blueprints/Widgets/WBP_DialoogUI.WBP_DialoogUI_C"))
  (bind _output_get (set `self.WBP_DialogueUIRef` _returnvalue))
  (`UserWidget.AddToViewport` _output_get 0)
  (bind _returnvalue_2 (`|CreateWidget` "/Game/Blueprints/Widgets/WBP_ManagerFeedback.WBP_ManagerFeedback_C"))
  (bind _output_get_2 (set `self.ManagerFeedbackWidget` _returnvalue_2))
  (`UserWidget.AddToViewport` _output_get_2 0)
  (`/Game/Blueprints/Widgets/WBP_ManagerFeedback.SetManagerFeedbackVisible` _output_get_2 false)
  (`PlayerController.SetViewTargetWithBlend` (`GameplayStatics.GetPlayerController` 0) (`self.Camera`) 0.0 "VTBlend_Linear" 0.0 false)
  (`self.SetActorHiddenInGame` (`GameplayStatics.GetPlayerCharacter` 0) true)
  (`self.CreateEndingScreenWidgetIfNeeded`))

(fn `CreateEndingScreenWidgetIfNeeded`
  (if (not (`KismetSystemLibrary.IsValid` (`self.EndScreenWidgetM1Ref`)))
    (bind _returnvalue (`|CreateWidget` "/Game/Blueprints/Widgets/WBP_EndScreenM1.WBP_EndScreenM1_C"))
    (bind _output_get (set `self.EndScreenWidgetM1Ref` _returnvalue))
    (`UserWidget.AddToViewport` _output_get 0)
    (`Widget.SetVisibility` _output_get "Collapsed")))

(fn `ShowEndingScreen`
  (`Widget.SetVisibility` (`self.EndScreenWidgetM1Ref`) "Visible"))

(fn `UserConstructionScript`)