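; Main player controller that shows the mouse cursor and switches between world interaction and UI modes.
; On BeginPlay it enables click and mouse-over events, then finds the BP_CameraPawn_Main actor and sets it as the view target.
; EnterUIMode sets CameraLocked and disables click and mouse-over events, and ExitUIMode reverses both.
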(event `self.ReceiveBeginPlay`
  (set `self.bShowMouseCursor` true)
  (set `self.bEnableClickEvents` true)
  (set `self.bEnableMouseOverEvents` true)
  (bind _returnvalue (`GameplayStatics.GetActorOfClass` "/Game/Blueprints/BP_CameraPawn_Main.BP_CameraPawn_Main_C"))
  (`self.SetViewTargetWithBlend` _returnvalue))

(fn `EnterUIMode`
  (set `self.bCameraLocked` true)
  (set `self.bEnableClickEvents` false)
  (set `self.bEnableMouseOverEvents` false))

(fn `ExitUIMode`
  (set `self.bCameraLocked` false)
  (set `self.bEnableClickEvents` true)
  (set `self.bEnableMouseOverEvents` true))

(fn `UserConstructionScript`)