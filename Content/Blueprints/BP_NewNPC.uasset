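; BP_NewNPC is an NPC that wanders endlessly between points supplied by the level's BP_NPCManager.
; On BeginPlay it finds the manager and randomizes its walk speed for variety.
; MoveToRandomPoint asks the manager for a random point other than the last target and walks there with AIMoveTo.
; It re-calls itself after a random pause on arrival, or after a short fixed delay on failure.
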(event `self.ReceiveBeginPlay`
  (bind _returnvalue (`GameplayStatics.GetActorOfClass` "/Game/Blueprints/BP_NPCManager.BP_NPCManager_C"))
  (set `self.NPCManagerRef` _returnvalue)
  (set `CharacterMovementComponent.MaxWalkSpeed` (`KismetMathLibrary.RandomFloatInRange` 140.0 190.0) (`self.CharacterMovement`))
  (`self.MoveToRandomPoint`))

(event `MoveToRandomPoint`
  (bind _randompoint (`/Game/Blueprints/BP_NPCManager.GetRandomNPCPointExcluding` (`self.NPCManagerRef`) (`self.LastTargetPoint`)))
  (bind _output_get (set `self.CurrentTargetPoint` _randompoint))
  (set `self.LastTargetPoint` _output_get)
  (`|AIMoveTo` self (0.0 0.0 0.0) (`self.CurrentTargetPoint`)
    (:`OnSuccess`
      (`KismetSystemLibrary.Delay` (`KismetMathLibrary.RandomFloatInRange` 2.0 5.0)))
    (:`OnFail`
      (`KismetSystemLibrary.Delay` 1.0)))
  (`self.MoveToRandomPoint`))

(fn `UserConstructionScript`)