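; Manager for the shelf-finding minigame: the player first unlocks every shelf, then helps customers one by one by choosing the requested shelf category.
; Timers drive press-and-hold on shelves with a progress ring, opening an info popup.
; DataTable rows script the manager tutorial, gating shelf clicks and advancing on matching wait types.
; It also owns the widgets, scores answers with feedback, tracks progress and shows the end screen.
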(event `self.ReceiveBeginPlay`
  (`GameplayStatics.PlaySound2D` "/Game/Sounds/WinkelWijs_ThemeSongMinigame2_Cue.WinkelWijs_ThemeSongMinigame2_Cue" 1.0 1.0 0.0 null null)
  (`self.InitializeReferences`)
  (`self.InitializeShelves`)
  (`self.InitializeWidgets`)
  (`self.StartManagerTutorial`))

(event `HandleCorrectShelf`
  (`GameplayStatics.PlaySound2D` "/Game/Sounds/S_CustomerHelpedRight_Cue.S_CustomerHelpedRight_Cue" 1.0 1.0 0.0 null null)
  (`/Game/Blueprints/Widgets/WBP_CustomerRequest.SetFeedbackText` (`self.CustomerRequestWidgetRef`) (`self.CorrectFeedbackText`))
  (`KismetSystemLibrary.Delay` 2.0)
  (`Widget.RemoveFromParent` (`self.CustomerRequestWidgetRef`))
  (set `self.CustomerRequestWidgetRef` null)
  (set `self.bRequestActive` false)
  (`/Game/Blueprints/BP_ClickableShelf.SetShelfDeselected` (`self.SelectedShelfRef`))
  (`self.AdvanceToNextCustomer`)
  (set `self.SelectedShelfRef` null))

(event `OnShelfHoldTimerFinished`
  (if (`self.bIsHoldingShelf`)
    (`self.CompleteShelfHoldAndOpenInfo`)))

(event `ShowHoldRingDelayed`
  (if (`self.bIsHoldingShelf`)
    (if (`KismetSystemLibrary.IsValid` (`self.ClickableShelfRef`))
      (`/Game/Blueprints/BP_ClickableShelf.ShowLoadingRing` (`self.ClickableShelfRef`) true)
      (bind _output_get (set `self.CurrentHoldProgress` (`KismetMathLibrary.FClamp` (+ (`self.CurrentHoldProgress`) (/ (`self.HoldVisualDelay`) (`self.HoldDuration`))))))
      (bind _aswbp_hold_ring (cast `/Game/Blueprints/Widgets/WBP_HoldRing` (`WidgetComponent.GetUserWidgetObject` (`/Game/Blueprints/BP_ClickableShelf.HoldRingComponent` (`self.ClickableShelfRef`)))))
      (`/Game/Blueprints/Widgets/WBP_HoldRing.UpdateHoldRing` _aswbp_hold_ring _output_get))))

(event `StartFirstCustomerPhase`
  (`KismetSystemLibrary.Delay` 5.0)
  (`self.InitializeCustomers`)
  (`self.HandleTutorialWaitProgress` "NewEnumerator8"))

(event `EndManagerDialogue`
  (`KismetSystemLibrary.Delay` 5.0)
  (`Widget.RemoveFromParent` (`self.ManagerTutorialWidgetRef`)))

(fn `AdvanceToNextCustomer`
  (if (`KismetSystemLibrary.IsValid` (`self.ActiveCustomerRef`))
    (`/Game/Blueprints/BP_CustomerBase.DeactivateCustomer` (`self.ActiveCustomerRef`))
    (bind _output_get (set `self.CurrentCustomerIndex` (+ (`self.CurrentCustomerIndex`) 1)))
    (if (< _output_get (`KismetArrayLibrary.Array_Length` (`self.CustomerHelpNPC's`)))
      (bind _output_get_2 (set `self.ActiveCustomerRef` (`|GetArrayItem` (`self.CustomerHelpNPC's`) (`self.CurrentCustomerIndex`))))
      (`/Game/Blueprints/BP_CustomerBase.ActivateCustomer` _output_get_2)
      (else
        (`KismetSystemLibrary.PrintString` "No more customers")
        (`self.ShowEndScreen`)))))

(fn `AdvanceTutorialRow`
  (if (`self.CurrentRowEndsDialogue`)
    (`Widget.RemoveFromParent` (`self.ManagerTutorialWidgetRef`))
    (else
      (set `self.CurrentTutorialIndex` (+ (`self.CurrentTutorialIndex`) 1))
      (`self.ShowCurrentTutorialRow`))))

(fn `CancelShelfHold`
  (`KismetSystemLibrary.K2_ClearAndInvalidateTimerHandle` (`self.HoldTimerHandle`))
  (`KismetSystemLibrary.K2_ClearAndInvalidateTimerHandle` (`self.HoldVisualTimerHandle`))
  (set `self.bIsHoldingShelf` false)
  (set `self.CurrentHoldProgress` 0.0)
  (set `self.bHoldCompleted` false)
  (if (`KismetSystemLibrary.IsValid` (`self.ClickableShelfRef`))
    (`/Game/Blueprints/BP_ClickableShelf.ShowLoadingRing` (`self.ClickableShelfRef`) false)
    (set `self.ClickableShelfRef` null)
    (else
      (set `self.ClickableShelfRef` null))))

(fn `CheckTutorialProgressAfterShelfUnlock`
  (bind _progressbarwidgetref (`self.ProgressBarWidgetRef`))
  (if (== (`KismetArrayLibrary.Array_Length` (`self.UnlockedShelves`)) (`KismetArrayLibrary.Array_Length` (`self.AllShelves`)))
    (set `self.bIsUnlockPhase` false)
    (`/Game/Blueprints/Widgets/WBP_ObjectiveProgress.ChangeProgressBar` _progressbarwidgetref)
    (`/Game/Blueprints/Widgets/WBP_ObjectiveProgress.UpdateProgressCustomer` _progressbarwidgetref 0 (`KismetArrayLibrary.Array_Length` (`self.CustomerHelpNPC's`)))
    (`self.HandleTutorialWaitProgress` "NewEnumerator2")
    (set `self.UnlockShelfRef` null)
    (`/Game/Blueprints/BP_ClickableShelf.SetShelfDeselected` (`self.SelectedShelfRef`))
    (`self.StartFirstCustomerPhase`)))

(fn `CompleteShelfHoldAndOpenInfo`
  (bind _shelfwidgetref (`self.ShelfWidgetRef`))
  (if (`self.bIsHoldingShelf`)
    (set `self.bHoldCompleted` true)
    (set `self.bIsHoldingShelf` false)
    (set `self.CurrentHoldProgress` 0.0)
    (`/Game/Blueprints/BP_ClickableShelf.ShowLoadingRing` (`self.ClickableShelfRef`) false)
    (`/Game/Blueprints/Widgets/WBP_ShelfInteraction.SetOwningShelf` _shelfwidgetref (`self.ClickableShelfRef`))
    (`/Game/Blueprints/Widgets/WBP_ShelfInteraction.ShowInfoPage` _shelfwidgetref)
    (`/Game/Blueprints/PlayerControllerMain.EnterUIMode` (`self.PlayerControllerRef`))
    (set `self.ShelfPopupIsOpen` true)
    (set `self.UnlockShelfRef` (`self.ClickableShelfRef`))
    (if (not (`self.bIsUnlockPhase`))
      (`self.HandleTutorialWaitProgress` "NewEnumerator4"))))

(fn `CompleteShelfUnlock`
  (bind _unlockshelfref (`self.UnlockShelfRef`))
  (if (not (`KismetArrayLibrary.Array_Contains` (`self.UnlockedShelves`) (`self.UnlockShelfRef`)))
    (`KismetArrayLibrary.Array_AddUnique` (`self.UnlockedShelves`) _unlockshelfref)
    (`/Game/Blueprints/BP_ClickableShelf.SetShelfUnlocked` _unlockshelfref)
    (`self.CheckTutorialProgressAfterShelfUnlock`)
    (`/Game/Blueprints/Widgets/WBP_ObjectiveProgress.UpdateProgressUnlock` (`self.ProgressBarWidgetRef`) (`KismetArrayLibrary.Array_Length` (`self.UnlockedShelves`)) (`KismetArrayLibrary.Array_Length` (`self.AllShelves`)))
    (`self.HandleTutorialWaitProgress` "NewEnumerator1")
    (set `self.IsCustomerTutorialActive` true)))

(fn `CreateEndScreenWidgetIfNeeded`
  (if (not (`KismetSystemLibrary.IsValid` (`self.EndScreenWidgetRef`)))
    (bind _returnvalue (`|CreateWidget` "/Game/Blueprints/Widgets/WBP_EndScreenM2.WBP_EndScreenM2_C"))
    (bind _output_get (set `self.EndScreenWidgetRef` _returnvalue))
    (`UserWidget.AddToViewport` _output_get 0)
    (`Widget.SetVisibility` _output_get "Collapsed")))

(fn `CreateHoldRingWidgetIfNeeded`
  (if (not (`KismetSystemLibrary.IsValid` (`self.HoldRingWidget`)))
    (bind _returnvalue (`|CreateWidget` "/Game/Blueprints/Widgets/WBP_HoldRing.WBP_HoldRing_C"))
    (set `self.HoldRingWidget` _returnvalue)))

(fn `CreateManagerTutorialWidgetIfNeeded`
  (if (not (`KismetSystemLibrary.IsValid` (`self.ManagerTutorialWidgetRef`)))
    (bind _returnvalue (`|CreateWidget` "/Game/Blueprints/Widgets/WBP_ManagerTutorial.WBP_ManagerTutorial_C"))
    (bind _output_get (set `self.ManagerTutorialWidgetRef` _returnvalue))
    (`UserWidget.AddToViewport` _output_get 0)
    (`Widget.SetVisibility` _output_get "Collapsed")))

(fn `CreateProgressBarWidgetIfNeeded`
  (if (not (`KismetSystemLibrary.IsValid` (`self.ProgressBarWidgetRef`)))
    (bind _returnvalue (`|CreateWidget` "/Game/Blueprints/Widgets/WBP_ObjectiveProgress.WBP_ObjectiveProgress_C"))
    (bind _output_get (set `self.ProgressBarWidgetRef` _returnvalue))
    (`UserWidget.AddToViewport` _output_get 10)
    (`/Game/Blueprints/Widgets/WBP_ObjectiveProgress.UpdateProgressUnlock` _output_get 0 (`KismetArrayLibrary.Array_Length` (`self.AllShelves`)))))

(fn `CreateShelfWidgetIfNeeded`
  (if (`KismetSystemLibrary.IsValid` (`self.ShelfWidgetRef`))
    (`self.ResetShelfWidgetState`)
    (else
      (bind _returnvalue (`|CreateWidget` "/Game/Blueprints/Widgets/WBP_ShelfInteraction.WBP_ShelfInteraction_C" null null))
      (bind _output_get (set `self.ShelfWidgetRef` _returnvalue))
      (`UserWidget.AddToViewport` _output_get 20)
      (`self.ResetShelfWidgetState`))))

(fn `HandleTutorialWaitProgress`
  (params (TriggeredWaitType :type "/Game/Blueprints/Enums/E_ManagerTutorialWaitType Enum" :default "NewEnumerator0"))
  (if (`|EnumEquality` TriggeredWaitType (`self.CurrentTutorialWaitType`))
    (`self.AdvanceTutorialRow`)))

(fn `InitializeCustomers`
  (set `self.CurrentCustomerIndex` 0)
  (if (> (`KismetArrayLibrary.Array_Length` (`self.CustomerHelpNPC's`)) 0)
    (for (_array_element _array_index) (`self.CustomerHelpNPC's`)
      (if (== _array_index (`self.CurrentCustomerIndex`))
        (set `self.ActiveCustomerRef` _array_element)
        (`/Game/Blueprints/BP_CustomerBase.ActivateCustomer` _array_element)
        (`KismetSystemLibrary.PrintString` "is begonnen!")
        (else
          (`/Game/Blueprints/BP_CustomerBase.DeactivateCustomer` _array_element))))))

(fn `InitializeReferences`
  (`|ExecutionSequence`
    (:`then_0`
      (bind _returnvalue (`GameplayStatics.GetActorOfClass` "/Game/Blueprints/PlayerControllerMain.PlayerControllerMain_C"))
      (set `self.PlayerControllerRef` _returnvalue))
    (:`then_1`
      (bind _returnvalue_2 (`GameplayStatics.GetActorOfClass` "/Game/Blueprints/BP_HelpCustomer.BP_HelpCustomer_C"))
      (set `self.HelpCustomerRef` _returnvalue_2))
    (:`then_2`
      (bind _outactors (`GameplayStatics.GetAllActorsOfClass` "/Game/Blueprints/BP_HelpCustomer.BP_HelpCustomer_C"))
      (bind _output_get (set `self.CustomerHelpNPC's` _outactors))
      (for _array_element _output_get
        (set `/Game/Blueprints/BP_CustomerBase.SchappenVindenManagerRef` self _array_element)))))

(fn `InitializeShelves`
  (set `self.bIsUnlockPhase` true)
  (bind _outactors (`GameplayStatics.GetAllActorsOfClass` "/Game/Blueprints/BP_ClickableShelf.BP_ClickableShelf_C"))
  (bind _output_get (set `self.AllShelves` _outactors))
  (for _array_element _output_get
    (`/Game/Blueprints/BP_ClickableShelf.SetShelfLocked` _array_element)))

(fn `InitializeWidgets`
  (`self.CreateManagerTutorialWidgetIfNeeded`)
  (`self.CreateShelfWidgetIfNeeded`)
  (`self.CreateHoldRingWidgetIfNeeded`)
  (`self.CreateEndScreenWidgetIfNeeded`)
  (`self.CreateProgressBarWidgetIfNeeded`))

(fn `JumpToTutorialRow`
  (params (BeginRowName :type Name))
  (set `self.CurrentTutorialIndex` (`KismetArrayLibrary.Array_Find` (`self.TutorialRowOrder`) BeginRowName))
  (`self.ShowCurrentTutorialRow`))

(fn `PositionHoldRingOnShelf`
  (`UserWidget.SetPositionInViewport` (`self.HoldRingWidget`) (- (`GameplayStatics.ProjectWorldToScreen` (`self.PlayerControllerRef`) (`SceneComponent.K2_GetComponentLocation` (`/Game/Blueprints/BP_ClickableShelf.HoldWidgetAnchor` (`self.ClickableShelfRef`)))) (`KismetMathLibrary.MakeVector2D` 40.0 40.0)) true))

(fn `ResetShelfWidgetState`
  (bind _shelfwidgetref (`self.ShelfWidgetRef`))
  (`/Game/Blueprints/Widgets/WBP_ShelfInteraction.SetConfirmEnabled` _shelfwidgetref false)
  (`/Game/Blueprints/Widgets/WBP_ShelfInteraction.ShowBevestigButton` _shelfwidgetref false))

(fn `SelectShelf`
  (params (ClickedShelf :type "/Game/Blueprints/BP_ClickableShelf Object Reference"))
  (bind _shelfwidgetref (`self.ShelfWidgetRef`))
  (bind _selectedshelfref (`self.SelectedShelfRef`))
  (if (not (== ClickedShelf _selectedshelfref))
    (`|ExecutionSequence`
      (:`then_0`
        (if (`KismetSystemLibrary.IsValid` _selectedshelfref)
          (`/Game/Blueprints/BP_ClickableShelf.SetShelfDeselected` _selectedshelfref)))
      (:`then_1`
        (set `self.SelectedShelfRef` ClickedShelf)
        (`/Game/Blueprints/BP_ClickableShelf.SetShelfSelected` _selectedshelfref)
        (`/Game/Blueprints/Widgets/WBP_ShelfInteraction.SetOwningShelf` _shelfwidgetref ClickedShelf)
        (`/Game/Blueprints/Widgets/WBP_ShelfInteraction.SetConfirmEnabled` _shelfwidgetref true)))))

(fn `SetAllShelvesClickable`
  (params (NewClickable :type Boolean))
  (for _array_element (`self.AllShelves`)
    (`/Game/Blueprints/BP_ClickableShelf.SetClickable` _array_element NewClickable)))

(fn `ShowCurrentTutorialRow`
  (locals (CurrentRowName :type Name))
  (bind _managertutorialwidgetref (`self.ManagerTutorialWidgetRef`))
  (bind _output_get (set `local.CurrentRowName` (`|GetArrayItem` (`self.TutorialRowOrder`) (`self.CurrentTutorialIndex`))))
  (set `self.CurrentTutorialWaitType` "NewEnumerator0")
  (bind _returnvalue (`|GetDataTableRow` "/Game/Blueprints/DataTables/DT_ManagerTutorialRowProduct.DT_ManagerTutorialRowProduct" _output_get)
    (:`then`
      (`GameplayStatics.PlaySound2D` "/Game/Sounds/S_ManagerNotification2_Cue.S_ManagerNotification2_Cue" 1.0 1.0 0.0 null null)
      (bind (_dialoguemanagertext _requirecontinueclick _waittype _endtutorialdialogue _setshelvesclickable _allowconfirmbutton _portrait) (break `/Game/Blueprints/DataTables/ST_ManagerTutorialRow` _returnvalue))
      (set `self.CurrentTutorialWaitType` _waittype)
      (set `self.CurrentRowEndsDialogue` _endtutorialdialogue)
      (`/Game/Blueprints/Widgets/WBP_ManagerTutorial.SetManagerDialogue` _managertutorialwidgetref _dialoguemanagertext)
      (`/Game/Blueprints/Widgets/WBP_ManagerTutorial.PlayAnimationPop` _managertutorialwidgetref)
      (`/Game/Blueprints/Widgets/WBP_ManagerTutorial.UpdateManagerPortrait` _managertutorialwidgetref _portrait)
      (`self.SetAllShelvesClickable` _setshelvesclickable)
      (`/Game/Blueprints/Widgets/WBP_ShelfInteraction.ShowBevestigButton` (`self.ShelfWidgetRef`) _allowconfirmbutton)
      (if (`self.CurrentRowEndsDialogue`)
        (`self.EndManagerDialogue`)))))

(fn `ShowEndScreen`
  (bind _endscreenwidgetref (`self.EndScreenWidgetRef`))
  (`GameplayStatics.PlaySound2D` "/Game/Sounds/S_LevelCompleted_Cue.S_LevelCompleted_Cue" 1.0 1.0 0.0 null null)
  (`/Game/Blueprints/PlayerControllerMain.EnterUIMode` (`self.PlayerControllerRef`))
  (`Widget.RemoveFromParent` (`self.ShelfWidgetRef`))
  (`Widget.RemoveFromParent` (`self.ProgressBarWidgetRef`))
  (`Widget.SetVisibility` _endscreenwidgetref "Visible")
  (`/Game/Blueprints/Widgets/WBP_EndScreenM2.PlayPopupAni` _endscreenwidgetref)
  (`/Game/Blueprints/Widgets/WBP_EndScreenM2.PlayStarAni` _endscreenwidgetref))

(fn `StartManagerTutorial`
  (set `self.CurrentTutorialIndex` 0)
  (`Widget.SetVisibility` (`self.ManagerTutorialWidgetRef`) "HitTestInvisible")
  (`self.ShowCurrentTutorialRow`))

(fn `StartShelfHold`
  (params (ClickedShelf :type "/Game/Blueprints/BP_ClickableShelf Object Reference"))
  (if (not (`self.ShelfPopupIsOpen`))
    (`KismetSystemLibrary.K2_ClearAndInvalidateTimerHandle` (`self.HoldTimerHandle`))
    (`KismetSystemLibrary.K2_ClearAndInvalidateTimerHandle` (`self.HoldVisualTimerHandle`))
    (`|ExecutionSequence`
      (:`then_0`
        (if (`KismetSystemLibrary.IsValid` (`self.ClickableShelfRef`))
          (`/Game/Blueprints/BP_ClickableShelf.ShowLoadingRing` (`self.ClickableShelfRef`) false)))
      (:`then_1`
        (set `self.ClickableShelfRef` ClickedShelf)
        (`self.SelectShelf` ClickedShelf)
        (set `self.bIsHoldingShelf` true)
        (set `self.bHoldCompleted` false)
        (set `self.CurrentHoldProgress` 0.0)
        (bind _returnvalue (`KismetSystemLibrary.K2_SetTimerDelegate` (`|CreateDelegate` :!event `OnShelfHoldTimerFinished`) (`self.HoldDuration`)))
        (set `self.HoldTimerHandle` _returnvalue)
        (bind _returnvalue_2 (`KismetSystemLibrary.K2_SetTimerDelegate` (`|CreateDelegate` :!event `ShowHoldRingDelayed`) (`self.HoldVisualDelay`) true))
        (set `self.HoldVisualTimerHandle` _returnvalue_2)))))

(fn `SubmitShelfChoice`
  (params (ChosenCategory :type "/Game/Blueprints/Enums/E_ShelfCategory Enum" :default "NewEnumerator0"))
  (bind _customerrequestwidgetref (`self.CustomerRequestWidgetRef`))
  (if (`self.bRequestActive`)
    (if (`|EnumEquality` (`self.ActiveTargetCategory`) ChosenCategory)
      (`self.HandleCorrectShelf`)
      (`/Game/Blueprints/Widgets/WBP_CustomerRequest.UpdatePFPHappy` _customerrequestwidgetref)
      (`/Game/Blueprints/Widgets/WBP_ObjectiveProgress.UpdateProgressCustomer` (`self.ProgressBarWidgetRef`) (+ (`self.CurrentCustomerIndex`) 1) (`KismetArrayLibrary.Array_Length` (`self.CustomerHelpNPC's`)))
      (if (and (`self.IsCustomerTutorialActive`) (`|EnumEquality` (`self.CurrentTutorialWaitType`) "NewEnumerator7"))
        (`self.JumpToTutorialRow` "CustomerHelp_Correct_01"))
      (else
        (`GameplayStatics.PlaySound2D` "/Game/Sounds/S_CustomerHelpedWrong_Cue.S_CustomerHelpedWrong_Cue" 1.0 1.0 0.0 null null)
        (`/Game/Blueprints/Widgets/WBP_CustomerRequest.SetFeedbackText` _customerrequestwidgetref (`self.WrongFeedbackText`))
        (`/Game/Blueprints/Widgets/WBP_CustomerRequest.UpdatePFPSad` _customerrequestwidgetref)
        (if (and (`self.IsCustomerTutorialActive`) (`|EnumEquality` (`self.CurrentTutorialWaitType`) "NewEnumerator7"))
          (`self.JumpToTutorialRow` "CustomerHelp_Wrong_01"))))))

(fn `UserConstructionScript`)