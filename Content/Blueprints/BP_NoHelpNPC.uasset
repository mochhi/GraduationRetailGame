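; BP_NoHelpNPC is an NPC that endlessly wanders between points supplied by BP_NPCManager.
; On BeginPlay it finds the manager and randomizes its walk speed.
; Each cycle releases its current point, reserves a random new one through the manager and walks there with AIMoveTo.
; It pauses for a random time on arrival, or retries after a short delay if the move fails or no valid point exists.
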(event `self.ReceiveBeginPlay`
  (bind _returnvalue (`GameplayStatics.GetActorOfClass` "/Game/Blueprints/BP_NPCManager.BP_NPCManager_C"))
  (set `self.NPCManagerRef_0` _returnvalue)
  (set `CharacterMovementComponent.MaxWalkSpeed` (`KismetMathLibrary.RandomFloatInRange` 120.0 150.0) (`self.CharacterMovement`))
  (`self.MoveToRandomPoint`))

(event `MoveToRandomPoint`
  (`/Game/Blueprints/BP_NPCManager.ReleaseNoHelpPoint` (`self.NPCManagerRef_0`) (`self.CurrentTargetPoint`))
  (bind _randompoint (`/Game/Blueprints/BP_NPCManager.GetRandomNPCPoint` (`self.NPCManagerRef_0`)))
  (if (`KismetSystemLibrary.IsValid` _randompoint)
    (`/Game/Blueprints/BP_NPCManager.ReserveNoHelpPoint` (`self.NPCManagerRef_0`) _randompoint)
    (set `self.CurrentTargetPoint` _randompoint)
    (`|AIMoveTo` self (0.0 0.0 0.0) (`self.CurrentTargetPoint`) 10.0
      (:`OnSuccess`
        (`KismetSystemLibrary.Delay` (`KismetMathLibrary.RandomFloatInRange` 5.0 7.0)))
      (:`OnFail`
        (`KismetSystemLibrary.Delay` 1.0)))
    (`self.MoveToRandomPoint`)
    (else
      (`KismetSystemLibrary.Delay` 1.0)
      (`self.MoveToRandomPoint`))))

(fn `UserConstructionScript`)