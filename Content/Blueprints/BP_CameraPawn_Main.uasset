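; BP_CameraPawn_Main is a camera pawn that pans around its starting position in response to the mouse cursor.
; BeginPlay caches the PlayerControllerMain reference and the base location.
; Unless that controller's CameraLocked is set, Tick converts the cursor's offset from viewport center into a scaled, inverted world XY offset from the base.
; VInterpTo eases the pawn toward that target each frame, keeping the base height.
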(event `self.ReceiveBeginPlay`
  (bind _returnvalue (`GameplayStatics.GetActorOfClass` "/Game/Blueprints/PlayerControllerMain.PlayerControllerMain_C"))
  (set `self.PlayerControllerRef` _returnvalue)
  (set `self.BaseLocation` (`self.K2_GetActorLocation`)))

(event `self.ReceiveTick`
  (params (DeltaSeconds :type "Float (single-precision)"))
  (bind (_locationx _locationy) (`PlayerController.GetMousePosition` (`GameplayStatics.GetPlayerController` 0)))
  (bind (_x _y) (`KismetMathLibrary.BreakVector2D` (`WidgetLayoutLibrary.GetViewportSize`)))
  (if (not (`/Game/Blueprints/PlayerControllerMain.bCameraLocked` (`self.PlayerControllerRef`)))
    (`self.K2_SetActorLocation` (`KismetMathLibrary.VInterpTo` (`self.K2_GetActorLocation`) (`KismetMathLibrary.MakeVector` (+ (* (- (/ _x 2.0) _locationx) 0.2) (.x (`self.BaseLocation`))) (+ (* (- (/ _y 2.0) _locationy) 0.2) (.y (`self.BaseLocation`))) (.z (`self.BaseLocation`))) DeltaSeconds 5.0))))

(fn `UserConstructionScript`)