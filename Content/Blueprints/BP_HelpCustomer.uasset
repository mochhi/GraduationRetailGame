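; Customer NPC that wanders between points in the level and eventually walks to an exit and is destroyed.
; On BeginPlay it finds BP_NPCManager and loads its request from a data table.
; Starting behaviour randomizes walk speed and begins a self-repeating AI move loop over non-help points from the manager, retrying on failure while CanMoveToPoint holds.
; WalkAwayAndDestroy unhides it, disables clicking and sends it to ExitPoint.
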(event `self.ReceiveBeginPlay`
  (bind _returnvalue (`GameplayStatics.GetActorOfClass` "/Game/Blueprints/BP_NPCManager.BP_NPCManager_C"))
  (set `self.NPCManagerRef_0` _returnvalue)
  (`self.LoadRequestFromDataTable`))

(event `MoveToRandomPoint`
  (if (`self.CanMoveToPoint`)
    (bind _randompoint (`/Game/Blueprints/BP_NPCManager.GetRandomNPCPointExcludingHelp` (`self.NPCManagerRef_0`) (`self.LastTargetPoint`)))
    (bind _output_get (set `self.CurrentTargetPoint` _randompoint))
    (set `self.LastTargetPoint` _output_get)
    (`|AIMoveTo` self (`self.K2_GetActorLocation` (`self.CurrentTargetPoint`)) null 70.0
      (:`OnSuccess`
        (`KismetSystemLibrary.Delay` (`KismetMathLibrary.RandomFloatInRange` 5.0 5.0)))
      (:`OnFail`
        (`KismetSystemLibrary.Delay` 1.0)))
    (if (`self.CanMoveToPoint`)
      (`self.MoveToRandomPoint`))))

(event `WalkAwayAndDestroy`
  (`self.SetActorHiddenInGame` false)
  (set `self.CanBeClicked` false)
  (`|AIMoveTo` self (0.0 0.0 0.0) (`self.ExitPoint`) 50.0
    (:`OnSuccess`
      (`self.K2_DestroyActor` self))))

(fn `StartCustomerBehavior!`
  (set `CharacterMovementComponent.MaxWalkSpeed` (`KismetMathLibrary.RandomFloatInRange` 150.0 170.0) (`self.CharacterMovement`))
  (`self.MoveToRandomPoint`))

(fn `StartCustomerBehaviour`
  (set `CharacterMovementComponent.MaxWalkSpeed` (`KismetMathLibrary.RandomFloatInRange` 150.0 170.0) (`self.CharacterMovement`))
  (`self.MoveToRandomPoint`)
  (`parent.StartCustomerBehaviour`))

(fn `UserConstructionScript`)