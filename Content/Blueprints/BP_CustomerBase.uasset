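; BP_CustomerBase is the base customer NPC for the SchappenVinden gameplay, with hover outline and click-to-help requests.
; Clicking outside the unlock phase, with no active request, passes its text and target category to BP_SchappenVindenManager.
; For BP_HelpCustomer children, it then stops AI movement, shows the request widget and advances the tutorial.
; It also provides DataTable request loading, show/hide activation and an empty StartCustomerBehavior hook.
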(event `self.ReceiveBeginPlay`
  (bind _returnvalue (`GameplayStatics.GetActorOfClass` "/Game/Blueprints/BP_SchappenVindenManager.BP_SchappenVindenManager_C"))
  (set `self.SchappenVindenManagerRef` _returnvalue)
  (bind _returnvalue_2 (`GameplayStatics.GetActorOfClass` "/Game/Blueprints/BP_NPCManager.BP_NPCManager_C"))
  (set `self.NPCManagerRef` _returnvalue_2))

(event `self.CapsuleComponent.OnClicked`
  (params (TouchedComponent :type "PrimitiveComponent Object Reference") (ButtonPressed :type "Key Structure"))
  (bind _schappenvindenmanagerref (`self.SchappenVindenManagerRef`))
  (bind _schappenvindenmanagerref_2 (`self.SchappenVindenManagerRef`))
  (if (not (`/Game/Blueprints/BP_SchappenVindenManager.bRequestActive` _schappenvindenmanagerref))
    (if (not (`/Game/Blueprints/BP_SchappenVindenManager.bIsUnlockPhase` _schappenvindenmanagerref))
      (set `/Game/Blueprints/BP_SchappenVindenManager.bRequestActive` true _schappenvindenmanagerref_2)
      (set `/Game/Blueprints/BP_SchappenVindenManager.ActiveRequestText` (`self.CurrentRequestText`) _schappenvindenmanagerref_2)
      (set `/Game/Blueprints/BP_SchappenVindenManager.ActiveTargetCategory` (`self.CurrentTargetCategory`) _schappenvindenmanagerref_2)
      (bind _asbp_help_customer (cast `/Game/Blueprints/BP_HelpCustomer` self))
      (set `/Game/Blueprints/BP_SchappenVindenManager.CurrentRequestCustomerRef` _asbp_help_customer (`self.SchappenVindenManagerRef`))
      (set `self.bIsWaiting` true)
      (set `self.CanMoveToPoint` false)
      (bind _asaicontroller (cast `AIController` (`self.GetController`)))
      (`Controller.StopMovement` _asaicontroller)
      (`self.CreateCustomerRequestWidget!`)
      (`/Game/Blueprints/BP_SchappenVindenManager.HandleTutorialWaitProgress` (`self.SchappenVindenManagerRef`) "NewEnumerator3"))))

(event `self.ReceiveActorBeginCursorOver`
  (`MeshComponent.SetOverlayMaterial` (`self.Mesh`) "/Game/Assets/M_OutlineHover.M_OutlineHover"))

(event `self.ReceiveActorEndCursorOver`
  (`MeshComponent.SetOverlayMaterial` (`self.Mesh`) null))

(fn `ActivateCustomer`
  (`self.SetActorHiddenInGame` false)
  (`self.SetActorEnableCollision` true)
  (`self.StartCustomerBehavior`))

(fn `CreateCustomerRequestWidget!`
  (bind _returnvalue (`|CreateWidget` "/Game/Blueprints/Widgets/WBP_CustomerRequest.WBP_CustomerRequest_C" null (`self.CurrentRequestText`) (`/Game/Blueprints/BP_SchappenVindenManager.CurrentRequestCustomerRef` (`self.SchappenVindenManagerRef`))))
  (bind _output_get (set `/Game/Blueprints/BP_SchappenVindenManager.CustomerRequestWidgetRef` _returnvalue (`self.SchappenVindenManagerRef`)))
  (`/Game/Blueprints/Widgets/WBP_CustomerRequest.UpdatePFPHappy` _output_get)
  (`UserWidget.AddToViewport` _output_get 0))

(fn `DeactivateCustomer`
  (`self.SetActorHiddenInGame` true)
  (`self.SetActorEnableCollision` false))

(fn `LoadRequestFromDataTable`
  (bind _returnvalue (`|GetDataTableRow` (`self.CustomerRequestDataTable`) (`self.RequestRowName`))
    (:`then`
      (bind (_requestid _requesttext _targetcategory) (break `/Game/Blueprints/DataTables/ST_CustomerRequest` _returnvalue))
      (set `self.CurrentRequestText` _requesttext)
      (set `self.CurrentTargetCategory` _targetcategory)
      (set `self.RequestAssigned` true))))

(fn `StartCustomerBehavior`)

(fn `UserConstructionScript`)